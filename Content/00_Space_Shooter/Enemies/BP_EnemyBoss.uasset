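; Boss enemy for the space shooter that takes hits from player ammo and keeps a movement vector and shot delay.
; Overlapping "Lateral" actors reverses the vector and shortens the delay toward a floor; no movement or firing logic appears here.
; Player and ammo overlaps play explosion effects, but only ammo costs life.
; At zero life it fires OnEnemyDestroy and calls both EnemyDestroyed and PlayerDead on SS_GameMode.
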(event `self.ReceiveBeginPlay`
  (`parent.ReceiveBeginPlay`)
  (set `self.MovementVector` (`self.GetActorRightVector`))
  (set `self.DelayShoot` 1.0))

(event `self.ReceiveActorBeginOverlap`
  (params (OtherActor :type "Actor Object Reference"))
  (bind _tags (`Actor.Tags` OtherActor))
  (bind _returnvalue (- (`self.DelayShoot`) 0.1))
  (if (`KismetArrayLibrary.Array_Contains` (`Actor.Tags` OtherActor) "Lateral")
    (set `self.MovementVector` (* (`self.MovementVector`) -1))
    (set `self.DelayShoot` _returnvalue)
    (if (<= _returnvalue 0.0)
      (set `self.DelayShoot` 0.1))
    (elif (`KismetArrayLibrary.Array_Contains` _tags "Player")
      ;[1 1 1] Explosion
      (`GameplayStatics.SpawnEmitterAtLocation` "/Game/StarterContent/Particles/P_Explosion.P_Explosion" (`self.K2_GetActorLocation`))
      (`GameplayStatics.PlaySound2D` "/Game/StarterContent/Audio/Explosion02.Explosion02" 1.0 1.0 0.0 null null)
      (elif (`KismetArrayLibrary.Array_Contains` _tags "PlayerAmmo")
        (`GameplayStatics.SpawnEmitterAtLocation` "/Game/StarterContent/Particles/P_Explosion.P_Explosion" (`self.K2_GetActorLocation`))
        (`GameplayStatics.PlaySound2D` "/Game/StarterContent/Audio/Explosion02.Explosion02" 1.0 1.0 0.0 null null)
        (set `self.Life` (- (`self.Life`) 1))
        (if (== (`self.Life`) 0)
          (`self.OnEnemyDestroy`)
          (bind _asss_game_mode (cast `/Game/00_Space_Shooter/SS_GameMode` (`GameplayStatics.GetGameMode`)))
          (`/Game/00_Space_Shooter/SS_GameMode.EnemyDestroyed` _asss_game_mode)
          (`/Game/00_Space_Shooter/SS_GameMode.PlayerDead` _asss_game_mode))))))

(fn `UserConstructionScript`
  (`parent.UserConstructionScript`))