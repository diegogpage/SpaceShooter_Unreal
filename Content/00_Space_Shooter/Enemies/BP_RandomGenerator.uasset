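; BP_RandomGenerator is the space shooter's enemy spawner, producing enemies until the boss appears.
; A Delay on Tick paces spawns at random SpawnPoint-tagged components, with the game mode Level influencing the choice between BP_EnemyBase and BP_EnemyH.
; CambioSpawnTime shortens the interval.
; SpawnBoss halts generation, spawns BP_EnemyBoss at Point3 and disables the player's rapid fire.
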(event `SpawnBoss`
  (set `self.GeneradorActivo` false)
  (`|SpawnActorFromClass` "/Game/00_Space_Shooter/Enemies/BP_EnemyBoss.BP_EnemyBoss_C" (`SceneComponent.K2_GetComponentToWorld` (`self.Point3`)) "Undefined" "MultiplyWithRoot" null null)
  ;[1 1 1] Quito disparo rapido para el boss
  (bind _outactors (`GameplayStatics.GetAllActorsOfClass` (`self.Player`)))
  (`/Game/00_Space_Shooter/Players/BP_SpaceS_Character.DesactivarVelDisparos` _outactors))

(event `self.ReceiveBeginPlay`
  ;[1 1 1] Genero enemigos hasta que salga el boss
)

(event `Spawn`
  ;[1 1 1] Genero enemigos hasta que salga el boss
  (if (`self.GeneradorActivo`)
    (`self.SpawnEnemy`)))

(event `self.ReceiveTick`
  (params (DeltaSeconds :type "Float (single-precision)"))
  (`KismetSystemLibrary.Delay` (`self.SpawnTime`))
  (`self.Spawn`)
  (bind _asss_game_mode (cast `/Game/00_Space_Shooter/SS_GameMode` (`GameplayStatics.GetGameMode`)))
  (set `self.SS Game Mode` _asss_game_mode))

(event `CambioSpawnTime`
  (set `self.SpawnTime` (- (`self.SpawnTime`) 0.25)))

(fn `GetClassToSpawn`
  (returns (Class :type "Actor Class Reference"))
  (if (<= (`KismetMathLibrary.RandomInteger` (`/Game/00_Space_Shooter/SS_GameMode.Level` (`self.SS Game Mode`))) 1)
    (return (select `int` 0 :`0` "/Game/00_Space_Shooter/Enemies/BP_EnemyBase.BP_EnemyBase_C" :`1` "/Game/00_Space_Shooter/Enemies/BP_EnemyH.BP_EnemyH_C" :!type "/Game/00_Space_Shooter/Enemies/BP_EnemyBase Class Reference"))
    (else
      ;[1 1 1] Si el nivel es mayor de 2, limito a 2 para que no me spawnee enemigos que no tengo
      (return (select `int` (`KismetMathLibrary.RandomInteger` 2) :`0` "/Game/00_Space_Shooter/Enemies/BP_EnemyBase.BP_EnemyBase_C" :`1` "/Game/00_Space_Shooter/Enemies/BP_EnemyH.BP_EnemyH_C" :!type "/Game/00_Space_Shooter/Enemies/BP_EnemyBase Class Reference")))))

(fn `SpawnEnemy`
  (returns (`AsBP Enemy Base` :type "/Game/00_Space_Shooter/Enemies/BP_EnemyBase Object Reference"))
  (bind _returnvalue (`self.GetComponentsByTag` "/Script/Engine.SceneComponent" "SpawnPoint"))
  (bind _class (`self.GetClassToSpawn`))
  (bind _returnvalue_2 (`|SpawnActorFromClass` _class (`SceneComponent.K2_GetComponentToWorld` (`|GetArrayItem` _returnvalue (`KismetMathLibrary.RandomInteger` (`KismetArrayLibrary.Array_Length` _returnvalue)))) "Undefined" "MultiplyWithRoot" null null))
  (bind _asbp_enemy_base (cast `/Game/00_Space_Shooter/Enemies/BP_EnemyBase` _returnvalue_2))
  (return _asbp_enemy_base))

(fn `UserConstructionScript`)