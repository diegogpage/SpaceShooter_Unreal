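; Player projectile for the space shooter that flies straight along its forward vector.
; Tick moves it by Speed scaled by delta time, without sweeping.
; Overlapping an actor tagged Enemy or Lateral destroys the projectile after a short delay; it applies no damage itself.
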(event `self.ReceiveActorBeginOverlap`
  (params (OtherActor :type "Actor Object Reference"))
  (if (`KismetArrayLibrary.Array_Contains` (`Actor.Tags` OtherActor) "Enemy")
    (`KismetSystemLibrary.Delay` 0.1 :!label _label)
    (`self.K2_DestroyActor`)
    (elif (`KismetArrayLibrary.Array_Contains` (`Actor.Tags` OtherActor) "Lateral")
      (goto _label))))

(event `self.ReceiveTick`
  (params (DeltaSeconds :type "Float (single-precision)"))
  (`self.K2_SetActorLocation` (+ (`self.K2_GetActorLocation`) (* (`self.GetActorForwardVector`) (* DeltaSeconds (`self.Speed`))))))

(fn `UserConstructionScript`)