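; BP_PowUp_Vidas is a lives ("Vidas") power-up pickup for the space shooter.
; Each tick, Move shifts it along MovementVector at Speed, scaled by delta time, with no sweep.
; Overlapping an actor tagged "Player" destroys the pickup; this Blueprint's graphs do not grant any lives themselves.
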(event `self.ReceiveActorBeginOverlap`
  (params (OtherActor :type "Actor Object Reference"))
  (if (`KismetArrayLibrary.Array_Contains` (`Actor.Tags` OtherActor) "Player")
    (`self.K2_DestroyActor`)))

(event `self.ReceiveTick`
  (params (DeltaSeconds :type "Float (single-precision)"))
  (`self.Move` DeltaSeconds))

(fn `Move`
  (params (DeltaTime :type "Float (double-precision)"))
  (`self.K2_SetActorLocation` (+ (`self.K2_GetActorLocation`) (* (* DeltaTime (`self.Speed`)) (`self.MovementVector`)))))

(fn `UserConstructionScript`)